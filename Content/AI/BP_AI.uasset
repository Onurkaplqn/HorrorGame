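; BP_AI is an enemy character that hunts the player and performs a jumpscare attack.
; PawnSensing sets a blackboard "seeingPlayer" flag, cleared by a looping timer, and sphere traces switch the head spotlight on or off.
; AttackPlayer plays a sound, disables input and runs a montage, then a trace hit applies damage and opens ThirdPersonMap.
; Taking damage briefly halts its movement, then shows the win widget.
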(event OnSeePawn(PawnSensing)
  (params (Pawn :type Pawn%20Object%20Reference))
  (bind _attack_trace_point2 (Variables|Default|GetAttack%20Trace%20Point2))
  (bind _attack_trace_point1 (Variables|Default|GetAttack%20Trace%20Point1))
  (bind _returnvalue (Transformation|GetWorldLocation _attack_trace_point1))
  (bind _returnvalue_2 (Transformation|GetWorldLocation _attack_trace_point2))
  (if (Actor|ActorHasTag Pawn "Player")
    (AI|Components|Blackboard|SetValueasBool (AI|GetBlackboard (AI|GetAIController self)) (Utilities|Name|MakeLiteralName "seeingPlayer") true)
    ;[0.15 0.15 0.15 0.5] KAFA IŞIĞI KIRMIZI
    (bind (_outhit _returnvalue_3) (Collision|SphereTraceForObjects _returnvalue_2 (+ _returnvalue_2 (* (Math|Vector|GetForwardVector (Transformation|GetWorldRotation _attack_trace_point2)) 2.5e+02)) 2e+02 (Utilities|Array|MakeArray "ObjectTypeQuery3") false 0 "None"))
    (if _returnvalue_3
      (Rendering|Components|Light|SetIntensity (Variables|Default|Getheadspot) 1e+04)
      (Variables|Default|Setisheadspoton true)
      (bind (_outhit_2 _returnvalue_4) (Collision|SphereTraceForObjects _returnvalue (+ _returnvalue (* (Math|Vector|GetForwardVector (Transformation|GetWorldRotation _attack_trace_point1)) 2.5e+02)) 2e+02 (Utilities|Array|MakeArray "ObjectTypeQuery3") false 0 "None"))
      (if _returnvalue_4
        (Rendering|Components|Light|SetIntensity (Variables|Default|Getheadspot) 0.0)
        (Variables|Default|Setisheadspoton true)))))

(event Custom|Attack%20Player
  (bind _returnvalue (Game|GetPlayerCharacter 0))
  (bind _attack_trace_point (Variables|Default|GetAttack%20Trace%20Point))
  (bind _returnvalue_2 (Transformation|GetWorldLocation _attack_trace_point))
  (if (not (Variables|Default|Getattacking?))
    (Audio|PlaySound2D "/Game/AI/Sounds/jumpscare-sound-effect_4M2WcDHg.jumpscare-sound-effect_4M2WcDHg" 2.5 1.0 0.0 0 0)
    (Variables|Default|Setattacking? true)
    (Utilities|Casting|CastToBP_FirstPersonCharacter _returnvalue)
    (Input|DisableInput _returnvalue 0)
    (Animation|Montage|PlayMontage (Variables|Character|GetMesh) "/Game/AI/retargetattackDouble_Dagger_Stab_Anim_Montage.retargetattackDouble_Dagger_Stab_Anim_Montage"
      (:OnCompleted
        (Variables|Default|Setattacking? false)
        (bind (_outhit _returnvalue_3) (Collision|SphereTraceForObjects _returnvalue_2 (+ _returnvalue_2 (* (Math|Vector|GetForwardVector (Transformation|GetWorldRotation _attack_trace_point)) 7e+01)) 8e+01 (Utilities|Array|MakeArray "ObjectTypeQuery3") false 0 "None"))
        (if _returnvalue_3
          (Game|Damage|ApplyDamage (.HitActor (Collision|BreakHitResult _outhit)) 1e+01 0 0)
          (Utilities|FlowControl|Delay 0.3)
          (Game|OpenLevel(byName) "ThirdPersonMap"))))))

(event Custom|Stop%20Seeing%20Player
  (AI|Components|Blackboard|SetValueasBool (AI|GetBlackboard (AI|GetAIController self)) (Utilities|Name|MakeLiteralName "seeingPlayer") false))

(event EventBeginPlay
  (Utilities|Time|SetTimerbyEvent (delegate Custom|Stop%20Seeing%20Player) 0.8 true))

(event Game|Damage|EventAnyDamage
  (params (Damage :type Float%20%28single-precision%29) (DamageType :type Damage%20Type%20Object%20Reference) (InstigatedBy :type Controller%20Object%20Reference) (DamageCauser :type Actor%20Object%20Reference))
  (Pawn|Components|CharacterMovement|DisableMovement (Variables|Character|GetCharacterMovement))
  (Utilities|FlowControl|Delay 2.0)
  (Pawn|Components|CharacterMovement|SetMovementMode (Variables|Character|GetCharacterMovement) "MOVE_Walking" 0)
  (bind _returnvalue (UserInterface|CreateWidget "/Game/UI/WB_Win.WB_Win_C"))
  (UserInterface|Viewport|AddtoViewport _returnvalue 0))

(fn ConstructionScript)