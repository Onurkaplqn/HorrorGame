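; BP_Weapon is a weapon pickup actor that equips the player's first-person character and then destroys itself.
; Its NewFunction event casts player 0's character to BP_FirstPersonCharacter and calls EquipWeapon; overlap is not handled here.
; On BeginPlay, a timeline drives GlowIntensity on a dynamic material instance of Material_001, created anew each update.
; That instance is never applied to a mesh, as the Sphere SetMaterial node is unconnected.
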(event Collision|EventActorBeginOverlap
  (params (OtherActor :type Actor%20Object%20Reference)))

(event EventTick
  (params (DeltaSeconds :type Float%20%28single-precision%29)))

(event EventNewFunction
  (bind _asbp_first_person_character (Utilities|Casting|CastToBP_FirstPersonCharacter (Game|GetPlayerCharacter 0)))
  (Default|EquipWeapon _asbp_first_person_character)
  (Actor|DestroyActor))

(event EventBeginPlay
  (bind _newtrack_0 (Timeline|Timeline Play)
    (:Update
      (bind _returnvalue (Rendering|Material|CreateDynamicMaterialInstance "/Game/Blueprints/StarFbx/Material_001.Material_001" "None" "None" :!class /Script/Engine.KismetMaterialLibrary))
      (Rendering|Material|SetScalarParameterValue _returnvalue "GlowIntensity" _newtrack_0 :!class /Script/Engine.MaterialInstanceDynamic))))

(fn ConstructionScript)